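; BP_Boid_Singleton_01 is a spawner actor that releases BP_Boid_01 boids from a rotating beacon, escalating over time.
; Tick turns BeaconRoot and calls SpawnBoids, which spawns at the beacon Sphere, facing outward from world origin, while the timer and population cap allow.
; Each boid receives singleton and Player references, active sparks and a follow coefficient that grows with spawn count.
; Each spawn shortens the interval down to a minimum.
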(event `self.ReceiveBeginPlay`
  (set `self.KilledBoids` 0))

(event `self.ReceiveTick`
  (params (DeltaSeconds :type "Float (single-precision)"))
  (`SceneComponent.K2_AddLocalRotation` (`self.BeaconRoot`) (`KismetMathLibrary.MakeRotator` 0.0 0.0 (`self.rotateDelta`)) false false)
  (`self.SpawnBoids`))

(fn `GetBeaconLocation`
  (returns (BeaconLoaction :type "Vector Structure"))
  (return (`SceneComponent.K2_GetComponentLocation` (`self.Sphere`))))

(fn `SpawnBoids`
  (locals (CurrentTime :type "Float (double-precision)") (NewBoid :type "/Game/BoidsAttack/Blueprints/BP_Boid_01 Object Reference"))
  (bind _returnvalue (- (`self.SecondsPerSpawn`) (`self.SpawnTimeDelta`)))
  (if (and (>= (- (`KismetSystemLibrary.GetGameTimeInSeconds`) (`self.LastSpawn`)) (`self.SecondsPerSpawn`)) (<= (`KismetArrayLibrary.Array_Length` (`self.Boids`)) (`self.MaxBoids`)))
    (bind _beaconloaction (`self.GetBeaconLocation`))
    (bind _returnvalue_2 (`|SpawnActorFromClass` "/Game/BoidsAttack/Blueprints/BP_Boid_01.BP_Boid_01_C" (`KismetMathLibrary.MakeTransform` _beaconloaction (`KismetMathLibrary.MakeRotFromX` (`KismetMathLibrary.Normal` _beaconloaction))) "Undefined" "OverrideRootScale" null null))
    (bind _output_get (set `local.NewBoid` _returnvalue_2))
    (`KismetArrayLibrary.Array_Add` (`self.Boids`) _output_get)
    (set `/Game/BoidsAttack/Blueprints/BP_Boid_01.Singleton` self (`local.NewBoid`))
    (set `/Game/BoidsAttack/Blueprints/BP_Boid_01.Player` (`self.Player`) (`local.NewBoid`))
    (set `self.LastSpawn` (`KismetSystemLibrary.GetGameTimeInSeconds`))
    (set `/Game/BoidsAttack/Blueprints/BP_Boid_01.Follow_Coef` (+ (`self.InitialFollowCoef`) (* (`self.FollowCoefDelta`) (`KismetMathLibrary.Conv_IntToDouble` (`self.SpawnedBoids`)))) (`local.NewBoid`))
    (`ActorComponent.Activate` (`/Game/BoidsAttack/Blueprints/BP_Boid_01.Sparks02` (`local.NewBoid`)) true)
    (`/Engine/EditorBlueprintResources/StandardMacros.IncrementInt` (`self.SpawnedBoids`)
      (:`  `
        (if (>= _returnvalue (`self.MinSpawnTime`))
          (set `self.SecondsPerSpawn` _returnvalue))))))

(fn `UserConstructionScript`)