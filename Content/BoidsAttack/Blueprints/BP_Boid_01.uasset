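; BP_Boid_01 is a flocking enemy that hunts the player and explodes.
; Each tick sums cohesion, separation, alignment, leader-follow and capsule-trace avoidance forces into its physics velocity.
; The leader, chosen by player proximity or line of sight, steers toward the visible player or a Singleton beacon.
; Projectile hits make it fall burning before exploding; player contact also triggers Kill, whose blast chains to nearby boids, kills the player and pushes physics objects.
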(event `self.ReceiveBeginPlay`
  (cast `/Game/BoidsAttack/PlayerStuff/FirstPersonCharacter_Boids` (`GameplayStatics.GetPlayerPawn` 0))
  (`self.SetBehaviorState` "NewEnumerator0"))

(event `self.ReceiveTick`
  (params (DeltaSeconds :type "Float (single-precision)"))
  (switch `/Game/BoidsAttack/Blueprints/E_BoidState_01` (`self.BehaviorState`)
    (:`NewEnumerator0`
      (`self.FindNeighbors` :!label _label)
      (`self.FindTarget`)
      (`self.GenerateFlockingForce`)
      (`self.SetRotation`))
    (:`NewEnumerator1`
      (goto _label))
    (:`NewEnumerator2`
      (`self.Kill`))))

(event `self.Collision_Sphere.OnComponentHit`
  (params (HitComponent :type "PrimitiveComponent Object Reference") (OtherActor :type "Actor Object Reference") (OtherComp :type "PrimitiveComponent Object Reference") (NormalImpulse :type "Vector Structure") (Hit :type "HitResult Structure (by ref)"))
  (bind _returnvalue (`GameplayStatics.GetObjectClass` OtherActor))
  (if (== _returnvalue "/Game/BoidsAttack/PlayerStuff/FirstPersonProjectile_Boids.FirstPersonProjectile_Boids_C")
    (`self.SetBehaviorState` "NewEnumerator2")
    (elif (== _returnvalue "/Game/BoidsAttack/PlayerStuff/FirstPersonCharacter_Boids.FirstPersonCharacter_Boids_C")
      (`self.Kill`))))

(event `self.NeighborRadius.OnComponentBeginOverlap`
  (params (OverlappedComponent :type "PrimitiveComponent Object Reference") (OtherActor :type "Actor Object Reference") (OtherComp :type "PrimitiveComponent Object Reference") (OtherBodyIndex :type Integer) (bFromSweep :type Boolean) (SweepResult :type "HitResult Structure (by ref)"))
  (bind _asstatic_mesh_actor (cast `StaticMeshActor` OtherActor))
  (`KismetArrayLibrary.Array_Add` (`self.StaticMeshNeighbors`) _asstatic_mesh_actor))

(event `self.NeighborRadius.OnComponentEndOverlap`
  (params (OverlappedComponent :type "PrimitiveComponent Object Reference") (OtherActor :type "Actor Object Reference") (OtherComp :type "PrimitiveComponent Object Reference") (OtherBodyIndex :type Integer))
  (bind _asstatic_mesh_actor (cast `StaticMeshActor` OtherActor))
  (`KismetArrayLibrary.Array_RemoveItem` (`self.StaticMeshNeighbors`) _asstatic_mesh_actor))

(fn `AmILeader`
  (returns (AmLeader :type Boolean))
  (`/Engine/EditorBlueprintResources/StandardMacros.IsValid` (`self.CurrentLeader`)
    (:`Is Valid`
      _)
    (:`Is Not Valid`
      (`self.DecideNewLeader`)))
  (return (== (`self.CurrentLeader`) self)))

(fn `DecideNewLeader`
  (locals (TargetLocation :type "Vector Structure") (ClosestDist :type "Float (double-precision)") (ClosestBoid :type "/Game/BoidsAttack/Blueprints/BP_Boid_01 Object Reference") (CurrentBoid :type "/Game/BoidsAttack/Blueprints/BP_Boid_01 Object Reference") (CurrentDist :type "Float (double-precision)"))
  (if (> (`self.N_Neighbors`) 0)
    (bind _output_get (set `local.TargetLocation` (`self.K2_GetActorLocation` (`self.Player`))))
    (set `local.ClosestDist` (`KismetMathLibrary.VSize` (- _output_get (`SceneComponent.K2_GetComponentLocation` (`self.Collision_Sphere`)))))
    (set `local.ClosestBoid` self)
    (for _array_element (`self.Neightbors`)
      (bind _output_get_2 (set `local.CurrentBoid` _array_element))
      (bind _output_get_3 (set `local.CurrentDist` (`KismetMathLibrary.VSize` (- (`self.K2_GetActorLocation` _output_get_2) (`local.TargetLocation`)))))
      (if (< _output_get_3 (`local.ClosestDist`))
        (set `local.ClosestBoid` (`local.CurrentBoid`))
        (set `local.ClosestDist` (`local.CurrentDist`))))
    (`self.SetLeader` (`local.ClosestBoid`))
    (else
      (set `self.CurrentLeader` self))))

(fn `FindNeighbors`
  (locals (Current :type "/Game/BoidsAttack/Blueprints/BP_Boid_01 Object Reference") (FoundLeader :type Boolean))
  (`KismetArrayLibrary.Array_Clear` (`self.Neightbors`))
  (for _array_element (`PrimitiveComponent.GetOverlappingActors` (`self.NeighborRadius`) null)
    (bind _asbp_boid_01 (cast `/Game/BoidsAttack/Blueprints/BP_Boid_01` _array_element))
    (bind _output_get (set `local.Current` _asbp_boid_01))
    (if (and (!= _output_get self) (`|EnumInequality` (`/Game/BoidsAttack/Blueprints/BP_Boid_01.BehaviorState` (`local.Current`)) "NewEnumerator2"))
      (`KismetArrayLibrary.Array_Add` (`self.Neightbors`) (`local.Current`))
      (if (and (not false) false)
        (set `local.FoundLeader` true))))
  (set `self.N_Neighbors` (`KismetArrayLibrary.Array_Length` (`self.Neightbors`)))
  (if (not false)
    (if (not (`local.FoundLeader`))
      (`self.DecideNewLeader`))
    (elif (`local.FoundLeader`)
      _)))

(fn `FindTarget`
  (locals (TargetAvailable :type Boolean) (HitDist :type "Float (double-precision)") (BeaconAvailable :type Boolean) (HeadLoc :type "Vector Structure"))
  (bind _headlocation (`/Game/BoidsAttack/PlayerStuff/FirstPersonCharacter_Boids.GetHeadLocation` (`self.Player`)))
  (set `local.HeadLoc` _headlocation)
  (for _array_element (`PrimitiveComponent.GetOverlappingActors` (`self.SightCone`) null)
    (if (== (`self.Player`) _array_element)
      (set `local.TargetAvailable` true)
      (break)))
  (if (`local.TargetAvailable`)
    (bind (_outhit _returnvalue) (`KismetSystemLibrary.LineTraceSingle` (`SceneComponent.K2_GetComponentLocation` (`self.Collision_Sphere`)) (`local.HeadLoc`) "TraceTypeQuery1" true :!label _label))
    (if _returnvalue
      (bind _output_get (set `local.HitDist` (`.Distance` (`GameplayStatics.BreakHitResult` _outhit))))
      (if (< _output_get (`KismetMathLibrary.VSize` (- (`SceneComponent.K2_GetComponentLocation` (`self.Collision_Sphere`)) (`local.HeadLoc`))))
        (set `self.CanSeeTarget` false)
        (else
          (set `self.CanSeeTarget` true)
          (if (not (`/Game/BoidsAttack/Blueprints/BP_Boid_01.CanSeeTarget` (`self.CurrentLeader`))) :!label _label_2
            (`self.SetLeader` self))))
      (else
        (set `self.CanSeeTarget` true)
        (goto _label_2)))
    (else
      (for _array_element_2 (`PrimitiveComponent.GetOverlappingActors` (`self.NeighborRadius`) null)
        (if (== (`self.Player`) _array_element_2)
          (set `local.TargetAvailable` true)
          (break)))
      (if (`local.TargetAvailable`)
        (goto _label)
        (else
          (set `self.CanSeeTarget` false))))))

(fn `GenerateAllignmentForce`
  (locals (TotalVelocity :type "Vector Structure"))
  (for _array_element (`self.Neightbors`)
    (set `local.TotalVelocity` (+ (`local.TotalVelocity`) (`SceneComponent.GetComponentVelocity` (`/Game/BoidsAttack/Blueprints/BP_Boid_01.Collision_Sphere` _array_element)))))
  (set `self.AllignmentForce` (* (/ (`local.TotalVelocity`) (`self.N_Neighbors`)) (`self.Allignment_Coef`))))

(fn `GenerateAvoidanceForce`
  (locals (CurrentLocation :type "Vector Structure") (Obstacle :type "Vector Structure") (Len :type "Float (double-precision)" :default 0.0))
  (set `local.CurrentLocation` (`SceneComponent.K2_GetComponentLocation` (`self.Collision_Sphere`)))
  (bind (_outhit _returnvalue) (`KismetSystemLibrary.CapsuleTraceSingleForObjects` (`local.CurrentLocation`) (* (`SceneComponent.GetForwardVector` (`self.Collision_Sphere`)) (`self.MaxSightDistance`)) 50.0 50.0 (`|MakeArray` "ObjectTypeQuery1" :!type "EObjectTypeQuery Enum")))
  (if _returnvalue
    (bind (_bblockinghit _binitialoverlap _time _distance _location _impactpoint _normal _impactnormal _physmat _hitactor) (`GameplayStatics.BreakHitResult` _outhit))
    (if (!= (`self.Player`) _hitactor)
      (bind _output_get (set `local.Obstacle` (- (`local.CurrentLocation`) _location)))
      (set `self.AvoidanceForce` (* (/ (`local.Obstacle`) (`KismetMathLibrary.VSizeSquared` _output_get)) (`self.Avoidance_Coef`))))))

(fn `GenerateCohesiveForce`
  (locals (Midpoint :type "Vector Structure"))
  (for _array_element (`self.Neightbors`)
    (set `local.Midpoint` (+ (`local.Midpoint`) (`self.K2_GetActorLocation` _array_element))))
  (bind _output_get (set `local.Midpoint` (/ (`local.Midpoint`) (`self.N_Neighbors`))))
  (set `self.CohesiveForce` (* (`KismetMathLibrary.Normal` (- _output_get (`SceneComponent.K2_GetComponentLocation` (`self.Collision_Sphere`)))) (`self.Cohesive_Coef`)))
  (return))

(fn `GenerateFlockingForce`
  (set `self.FlockingForce` (0.0 0.0 0.0))
  (set `self.CohesiveForce` (0.0 0.0 0.0))
  (set `self.AllignmentForce` (0.0 0.0 0.0))
  (set `self.FollowForce` (0.0 0.0 0.0))
  (set `self.AvoidanceForce` (0.0 0.0 0.0))
  (if (> (`self.N_Neighbors`) 0)
    (`self.GenerateCohesiveForce`)
    (`self.GenerateSeparationForce`)
    (`self.GenerateAllignmentForce`))
  (`self.GenerateFollowForce`)
  (`self.GenerateAvoidanceForce`)
  (bind _output_get (set `self.FlockingForce` (+ (`self.CohesiveForce`) (`self.SeparationForce`) (`self.AllignmentForce`) (`self.FollowForce`) (`self.AvoidanceForce`))))
  (`PrimitiveComponent.SetPhysicsLinearVelocity` (`self.Collision_Sphere`) _output_get false "None"))

(fn `GenerateFollowForce`
  (bind _amleader (`self.AmILeader`))
  (if _amleader
    (if (`self.CanSeeTarget`)
      (set `self.FollowForce` (- (`self.K2_GetActorLocation` (`self.Player`)) (`SceneComponent.K2_GetComponentLocation` (`self.Collision_Sphere`))))
      (else
        (bind _beaconloaction (`/Game/BoidsAttack/Blueprints/BP_Boid_Singleton_01.GetBeaconLocation` (`self.Singleton`)))
        (set `self.FollowForce` (- _beaconloaction (`SceneComponent.K2_GetComponentLocation` (`self.Collision_Sphere`))))))
    (set `self.FollowForce` (* (`KismetMathLibrary.Normal` (`self.FollowForce`)) (`self.Follow_Coef`)))
    (else
      (set `self.FollowForce` (0.0 0.0 0.0)))))

(fn `GenerateSeparationForce`
  (locals (AwayFrom :type "Vector Structure") (CurrentLocation :type "Vector Structure"))
  (set `local.CurrentLocation` (`SceneComponent.K2_GetComponentLocation` (`self.Collision_Sphere`)))
  (for _array_element (`self.Neightbors`)
    (set `local.AwayFrom` (+ (`local.AwayFrom`) (- (`local.CurrentLocation`) (`self.K2_GetActorLocation` _array_element)))))
  (set `self.SeparationForce` (* (`KismetMathLibrary.Normal` (`local.AwayFrom`)) (`self.Separation_Coef`))))

(fn `Kill`
  (locals (CurrentComponent :type "PrimitiveComponent Object Reference") (ImpulseDirection :type "Vector Structure"))
  (bind _p_mid_explosion_v3 (`self.P_Mid_Explosion_v3`))
  (if (>= (`KismetSystemLibrary.GetGameTimeInSeconds`) (+ (`self.TimeKilled`) (`self.DeathDuration`)))
    (`KismetArrayLibrary.Array_RemoveItem` (`/Game/BoidsAttack/Blueprints/BP_Boid_Singleton_01.Boids` (`self.Singleton`)) self)
    (`SceneComponent.K2_SetWorldRotation` :`self` _p_mid_explosion_v3)
    (if (not (`ActorComponent.IsActive` _p_mid_explosion_v3))
      (`ActorComponent.Activate` (`self.P_Mid_Explosion_v3`) false)
      (`SceneComponent.SetVisibility` (`self.StaticMesh`) false false)
      (`ActorComponent.Deactivate` (`self.Fire`))
      (`GameplayStatics.PlaySoundAtLocation` "/Game/BoidsAttack/SoundEffects/explosion01.explosion01" (`SceneComponent.K2_GetComponentLocation` (`self.Collision_Sphere`)) (struct) 1.0 1.0 0.0 null null null)
      (set `self.ExplosionTime` (`KismetSystemLibrary.GetGameTimeInSeconds`))
      (`PrimitiveComponent.SetSimulatePhysics` (`self.Collision_Sphere`) false)
      (`PrimitiveComponent.SetCollisionResponseToAllChannels` (`self.Collision_Sphere`) "ECR_Ignore")
      (for _array_element (`PrimitiveComponent.GetOverlappingActors` (`self.NeighborRadius`) null)
        (bind _asbp_boid_01 (cast `/Game/BoidsAttack/Blueprints/BP_Boid_01` _array_element)
          (:`then`
            (`self.SetBehaviorState` _asbp_boid_01 "NewEnumerator2"))
          (:`CastFailed`
            (if (== _array_element (`self.Player`))
              (`/Game/BoidsAttack/PlayerStuff/FirstPersonCharacter_Boids.KillPlayer` (`self.Player`))))))
      (for _array_element_2 (`PrimitiveComponent.GetOverlappingComponents` (`self.NeighborRadius`))
        (bind _output_get (set `local.CurrentComponent` _array_element_2))
        (if (`SceneComponent.IsSimulatingPhysics` _output_get "None")
          (bind _output_get_2 (set `local.ImpulseDirection` (- (`SceneComponent.K2_GetComponentLocation` (`local.CurrentComponent`)) (`SceneComponent.K2_GetComponentLocation` (`self.Collision_Sphere`)))))
          (bind _output_get_3 (set `local.ImpulseDirection` (`KismetMathLibrary.Normal` _output_get_2)))
          (`PrimitiveComponent.AddImpulse` (`local.CurrentComponent`) (* _output_get_3 (`self.ExplosiveForce_Coef`)) "None" true)))
      (elif (>= (- (`KismetSystemLibrary.GetGameTimeInSeconds`) (`self.ExplosionTime`)) (`self.ExplosionLength`))
        (`self.K2_DestroyActor`)))))

(fn `SetBehaviorState`
  (params (NewState :type "/Game/BoidsAttack/Blueprints/E_BoidState_01 Enum" :default "NewEnumerator0"))
  (bind _output_get (set `self.BehaviorState` NewState))
  (switch `/Game/BoidsAttack/Blueprints/E_BoidState_01` _output_get
    (:`NewEnumerator2`
      (`PrimitiveComponent.SetEnableGravity` (`self.Collision_Sphere`) true)
      (bind _returnvalue (`PrimitiveComponent.GetPhysicsLinearVelocity` (`self.Collision_Sphere`) "None"))
      (`PrimitiveComponent.SetPhysicsLinearVelocity` (`self.Collision_Sphere`) (`KismetMathLibrary.MakeVector` (.x _returnvalue) (.y _returnvalue)) false "None")
      (set `self.TimeKilled` (`KismetSystemLibrary.GetGameTimeInSeconds`))
      (`ActorComponent.Activate` (`self.Hit`) false)
      (`ActorComponent.Activate` (`self.Fire`) false)
      (`/Engine/EditorBlueprintResources/StandardMacros.IncrementInt` (`/Game/BoidsAttack/Blueprints/BP_Boid_Singleton_01.KilledBoids` (`self.Singleton`))
        (:`  `
          (`GameplayStatics.PlaySoundAtLocation` "/Game/StarterContent/Audio/Explosion01.Explosion01" (`SceneComponent.K2_GetComponentLocation` (`self.Collision_Sphere`)) (struct) 1.0 1.0 0.0 null null null))))))

(fn `SetLeader`
  (params (NewLeader :type "/Game/BoidsAttack/Blueprints/BP_Boid_01 Object Reference"))
  (set `self.CurrentLeader` NewLeader)
  (for _array_element (`self.Neightbors`)
    (set `/Game/BoidsAttack/Blueprints/BP_Boid_01.CurrentLeader` (`self.CurrentLeader`) _array_element)))

(fn `SetRotation`
  (locals (RotateTo :type "Vector Structure"))
  (if (or (`self.CanSeeTarget`) (and (`KismetSystemLibrary.IsValid` (`self.CurrentLeader`)) (`/Game/BoidsAttack/Blueprints/BP_Boid_01.CanSeeTarget` (`self.CurrentLeader`))))
    (bind _headlocation (`/Game/BoidsAttack/PlayerStuff/FirstPersonCharacter_Boids.GetHeadLocation` (`self.Player`)))
    (set `local.RotateTo` (`KismetMathLibrary.Normal` (- _headlocation (`SceneComponent.K2_GetComponentLocation` (`self.Collision_Sphere`)))))
    (else
      (set `local.RotateTo` (`self.FlockingForce`))))
  (`SceneComponent.K2_SetWorldRotation` (`self.Collision_Sphere`) (`KismetMathLibrary.MakeRotFromX` (`KismetMathLibrary.VLerp` (`self.GetActorForwardVector`) (`KismetMathLibrary.Normal` (`local.RotateTo`)) 0.25)) false false))

(fn `UserConstructionScript`)